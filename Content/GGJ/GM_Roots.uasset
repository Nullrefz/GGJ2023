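; GM_Roots is a game mode that sets up characters and a moving camera when play begins.
; It spawns NumberOfPlayers BP_Character pawns at a single PlayerStart, then has player controller 0 possess one.
; It records that controller in Players, spawns a BP_Camera at the possessed pawn's transform and calls StartMoving on it after a short delay.
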(event `self.ReceiveBeginPlay`
  (bind _returnvalue (`GameplayStatics.GetPlayerController` 0))
  (`self.SpawnPlayers`)
  (`KismetArrayLibrary.Array_Add` (`self.players`) _returnvalue)
  (bind _returnvalue_2 (`|SpawnActorFromClass` "/Game/GGJ/BP_Camera.BP_Camera_C" (`self.GetTransform` (`Controller.K2_GetPawn` _returnvalue)) "Undefined" "OverrideRootScale" null null))
  (`KismetSystemLibrary.Delay` 0.2)
  (`/Game/GGJ/BP_Camera.StartMoving` _returnvalue_2))

(fn `SpawnPlayers`
  (locals (PlayerStart :type "PlayerStart Object Reference"))
  (bind _returnvalue (`GameplayStatics.GetActorOfClass` "/Script/Engine.PlayerStart"))
  (`/Engine/EditorBlueprintResources/StandardMacros.IsValid` _returnvalue
    (:`Is Valid`
      (bind _output_get (set `local.PlayerStart` _returnvalue))
      (for _ (range 1 (+ (`self.NumberOfPlayers`) 1))
        (bind _returnvalue_2 (`|SpawnActorFromClass` "/Game/GGJ/BP_Character.BP_Character_C" (`self.GetTransform` _output_get) "AdjustIfPossibleButAlwaysSpawn" "OverrideRootScale" null null)))
      (`Controller.Possess` (`GameplayStatics.GetPlayerController` 0) _returnvalue_2))))

(fn `UserConstructionScript`)