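; BP_Camera is a camera actor that becomes player 0's view target and can follow that player's pawn.
; On BeginPlay it caches the GM_Roots game mode and sets itself as the view target of the first entry in its Players array.
; StartMoving, which nothing in this graph calls, starts a fast looping timer that snaps the actor to the pawn's location without interpolation, in place of Tick.
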(event `self.ReceiveBeginPlay`
  (bind _asgm_roots (cast `/Game/GGJ/GM_Roots` (`GameplayStatics.GetGameMode`)))
  (set `self.gamemode` _asgm_roots)
  (`PlayerController.SetViewTargetWithBlend` (`|GetArrayItem` (`/Game/GGJ/GM_Roots.players` (`self.gamemode`))) self 0.0 "VTBlend_EaseOut" 0.0 false))

(event `StartMoving`
  (bind _returnvalue (`KismetSystemLibrary.K2_SetTimerDelegate` (delegate `MoveCamera`) 0.01 true))
  (set `self.moveHandle` _returnvalue))

(event `MoveCamera`
  (`self.K2_SetActorLocation` (`self.K2_GetActorLocation` (`Controller.K2_GetPawn` (`|GetArrayItem` (`/Game/GGJ/GM_Roots.players` (`self.gamemode`)))))))

(fn `UserConstructionScript`)